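; Enemy character Blueprint with a floating health bar, footstep effects and weapon pickup on capsule overlap.
; Tick updates the HP widget from current and max HP and yaws it toward the player camera.
; Foot trigger functions fire events that trace down to spawn footprint decals and select a sound by surface type, with both feet passing Left to the sound.
; Construction assigns weapon, shield, body and blood components to variables.
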(event `self.ReceiveTick`
  (params (DeltaSeconds :type "Float (single-precision)"))
  (`self.ModifyHPValue`)
  (`self.RotateHPBar`))

(event `RightFoot`
  (`self.FootPrint` (`self.Right`))
  (`self.FootSound` (`self.Left`) :!label _label))

(event `LeftFoot`
  (`self.FootPrint` (`self.Left`))
  (goto _label))

(event `self.CapsuleComponent.OnComponentBeginOverlap`
  (params (OverlappedComponent :type "PrimitiveComponent Object Reference") (OtherActor :type "Actor Object Reference") (OtherComp :type "PrimitiveComponent Object Reference") (OtherBodyIndex :type Integer) (bFromSweep :type Boolean) (SweepResult :type "HitResult Structure (by ref)"))
  (`self.pickUpWeapon` OtherComp))

(fn `FootPrint`
  (params (Target :type "SceneComponent Object Reference"))
  (bind _returnvalue (`SceneComponent.K2_GetComponentLocation` Target))
  (bind _outhit (`KismetSystemLibrary.LineTraceSingle` (+ _returnvalue (0.0 0.0 20.0)) (- _returnvalue (0.0 0.0 20.0)) "TraceTypeQuery1"))
  (`GameplayStatics.SpawnDecalAtLocation` "/Game/Other/FootPrint.FootPrint" (20.0 20.0 20.0) (`.Location` (`GameplayStatics.BreakHitResult` _outhit)) (`KismetMathLibrary.MakeRotator` -90.0 90.0 (.yaw (`SceneComponent.K2_GetComponentRotation` Target))))
  (return))

(fn `FootSound`
  (params (self2 :type "ActorComponent Object Reference"))
  (bind _returnvalue (`self.K2_GetActorLocation` (`ActorComponent.GetOwner` self2)))
  (bind (_outhit _returnvalue_2) (`KismetSystemLibrary.LineTraceSingle` _returnvalue (- _returnvalue (0.0 0.0 300.0)) "TraceTypeQuery1"))
  (if _returnvalue_2
    (`GameplayStatics.PlaySoundAtLocation` (select `EPhysicalSurface` (`GameplayStatics.GetSurfaceType` _outhit) :!type "SoundBase Object Reference") (`.Location` (`GameplayStatics.BreakHitResult` _outhit))))
  (return))

(fn `LeftFootTrigger`
  (`self.LeftFoot`))

(fn `ModifyHPValue`
  (bind _currenthp (`self.CurrentHp`))
  (bind _asenemy_hpbar (cast `/Game/Blueprints/HPBar/EnemyHPBar` (`WidgetComponent.GetUserWidgetObject` (`self.Widget`))))
  (if (>= _currenthp 0.0)
    (`ProgressBar.SetPercent` (`/Game/Blueprints/HPBar/EnemyHPBar.ProgressBar_0` _asenemy_hpbar) (/ _currenthp (`self.MaxHp`)))))

(fn `RightFootTrigger`
  (`self.RightFoot`))

(fn `RotateHPBar`
  (bind _scene (`self.Scene`))
  (`SceneComponent.K2_SetWorldRotation` _scene (`KismetMathLibrary.MakeRotator` 0.0 0.0 (.yaw (`KismetMathLibrary.FindLookAtRotation` (`SceneComponent.K2_GetComponentLocation` _scene) (`PlayerCameraManager.GetCameraLocation` (`GameplayStatics.GetPlayerCameraManager` 0))))) false false))

(fn `UserConstructionScript`
  (set `self.WeaponCollider` (`self.Box`))
  (set `self.WeapondWrap` (`self.WeaponWrapper`))
  (set `self.shieldWrap` (`self.ShieldWrapper`))
  (set `self.characterBody` (`self.CapsuleComponent`))
  (set `self.Blood` "/Game/Environment/Effects/particles/Blood.Blood"))